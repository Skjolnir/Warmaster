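; Unit system that pools, spawns and respawns Blue and Red AI units for matches between two team behavior trees.
; Match start fills the pools once and teleports units to team PlayerStarts, temporarily tagged "Taken" to avoid reuse; match end re-pools active units.
; DamageSystem kills send units back to their team's pool location and queue them for a looping respawn timer.
; SetupNewTest destroys all units and swaps both behavior trees.
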(event `Setup Spawn Handling`
  (bind _outactors (`GameplayStatics.GetAllActorsOfClass` "/Game/05_World/WM_ActorPool.WM_ActorPool_C"))
  (for _array_element _outactors
    (`|SwitchGameplayTagContainer` (`/Game/00_Base/Systems/Components/WM_TeamComponent.TeamTag` (`/Game/05_World/WM_ActorPool.WM_TeamComponent` _array_element))
      (:`(GameplayTags=((TagName="Team.Blue")))`
        (set `self.PoolSpawnBlue` _array_element))
      (:`(GameplayTags=((TagName="Team.Red")))`
        (set `self.PoolSpawnRed` _array_element)))))

(event `Setup Respawn Handling`
  (`KismetSystemLibrary.K2_SetTimerDelegate` (delegate `Respawn Queue`) 5.0 true))

(event `self.ReceiveBeginPlay`
  (`self.Setup Match Handling`)
  (`self.Setup Spawn Handling`)
  (`self.Setup Damage Handling`)
  (`self.Setup Respawn Handling`))

(event `Respawn Queue`
  (`self.HandleRespawn`))

(event `Setup Match Handling`
  ;[1 1 1] Match Handling
  (bind _output_get (set `self.MatchSystem` (`Actor.GetComponentByClass` (`GameplayStatics.GetGameMode`) "/Game/00_Base/Systems/BP_WMMatchSystem.BP_WMMatchSystem_C")))
  (`/Engine/EditorBlueprintResources/StandardMacros.IsValid` _output_get
    (:`Is Valid`
      (add `WMMatchSystem.StartMatch` (`self.MatchSystem`) (delegate `Event Start Match`))
      (add `WMMatchSystem.EndMatch` (`self.MatchSystem`) (delegate `Event End Match`)))
    (:`Is Not Valid`
      (`KismetSystemLibrary.PrintString` "*** Game Mode has no \"WMMatchSystem\" component ***"))))

(event `Setup Damage Handling`
  ;[1 1 1] Damage Handling
  (bind _output_get (set `self.DamageSystem` (`Actor.GetComponentByClass` (`GameplayStatics.GetGameMode`) "/Script/Warmaster.WMDamageSystem")))
  (`/Engine/EditorBlueprintResources/StandardMacros.IsValid` _output_get
    (:`Is Valid`
      (add `self.ActorKilled` (delegate `Event Actor Killed`)))
    (:`Is Not Valid`
      (`KismetSystemLibrary.PrintString` "*** No DamageSystem found ***"))))

(event `Event Start Match`
  ;[1 1 1] Match Handling
  (`self.HandleStartMatch`))

(event `Event Actor Killed` :!signature `self.ActorKilled`
  (params (Actor :type "Actor Object Reference") (Killer :type "Actor Object Reference"))
  ;[1 1 1] Damage Handling
  (bind _pooledactor (`self.PoolActor` Actor))
  (`KismetArrayLibrary.Array_AddUnique` (`self.RespawnQueue`) _pooledactor))

(event `Event End Match`
  ;[1 1 1] Match Handling
  (`self.HandleEndMatch`))

(fn `ChooseRandomUnitName`
  (returns (RandomUnitName :type String))
  (locals (Name :type String) (Index :type Integer :default 0))
  (set `local.Index` (`KismetMathLibrary.RandomIntegerInRange` 0 (- (`KismetArrayLibrary.Array_Length` (`self.ActorNamePool`)) 1)))
  (set `local.Name` (`|GetArrayItem` (`self.ActorNamePool`) (`local.Index`)))
  (`KismetArrayLibrary.Array_Remove` (`self.ActorNamePool`) (`local.Index`))
  (return (`local.Name`)))

(fn `FillActorPools`
  (returns (WasSuccessful :type Boolean))
  (locals (Successful :type Boolean :default true) (NameCount :type Integer :default 0))
  (for _index (range 1 (+ (* (`self.ActorsPerTeam`) 2) 1))
    (if (== (mod _index 2) 0)
      (bind _pooledactor (`self.PoolActor` null (struct :`GameplayTags` (struct :`(TagName` "Team.Blue")))))
      (`/Engine/EditorBlueprintResources/StandardMacros.IsValid` _pooledactor
        (:`Is Valid`
          (`KismetArrayLibrary.Array_AddUnique` (`self.ActorPoolBlue`) _pooledactor))
        (:`Is Not Valid`
          (`KismetSystemLibrary.PrintString` "*** Pool Actor Creation failed ***")
          (set `local.Successful` false)))
      (else
        (bind _pooledactor_2 (`self.PoolActor` null (struct :`GameplayTags` (struct :`(TagName` "Team.Red")))))
        (`/Engine/EditorBlueprintResources/StandardMacros.IsValid` _pooledactor_2
          (:`Is Valid`
            (`KismetArrayLibrary.Array_AddUnique` (`self.ActorPoolRed`) _pooledactor_2))
          (:`Is Not Valid`
            (`KismetSystemLibrary.PrintString` "*** Pool Actor Creation failed ***")
            (set `local.Successful` false))))))
  (return (`local.Successful`)))

(fn `FindSpawn`
  (params (Team :type "GameplayTagContainer Structure"))
  (returns (Spawn :type "/Game/00_Base/WM_PlayerStart Object Reference"))
  (locals (TeamString :type String) (PlayerStart :type "Actor Object Reference"))
  (`|SwitchGameplayTagContainer` Team
    (:`(GameplayTags=((TagName="Team.Blue")))`
      (set `local.TeamString` "Blue"))
    (:`(GameplayTags=((TagName="Team.Red")))`
      (set `local.TeamString` "Red")))
  (bind _output_get (set `local.PlayerStart` (`GameModeBase.K2_FindPlayerStart` (`GameplayStatics.GetGameMode`) (`GameplayStatics.GetPlayerController` 0) (`local.TeamString`))))
  (`/Engine/EditorBlueprintResources/StandardMacros.IsValid` _output_get
    (:`Is Valid`
      (bind _aswm_player_start (cast `/Game/00_Base/WM_PlayerStart` (`local.PlayerStart`)))
      (return _aswm_player_start))
    (:`Is Not Valid`
      (`KismetSystemLibrary.PrintString` "*** FindPlayerStart returning invalid spawn ***")
      (return null))))

(fn `HandleEndMatch`
  (locals (ActorsToPool :type "Array of Actor Object Reference"))
  (`KismetArrayLibrary.Array_Clear` (`self.RespawnQueue`))
  (`KismetArrayLibrary.Array_Append` (`local.ActorsToPool`) (`self.ActiveNormalActors`))
  (`KismetArrayLibrary.Array_Append` (`local.ActorsToPool`) (`self.ActiveExtendedActors`))
  (for _array_element (`local.ActorsToPool`)
    (`self.PoolActor` _array_element)))

(fn `HandleRespawn`
  (locals (ActorsToRespawn :type "Array of Actor Object Reference") (DebugString :type String :default "*** UnitSystem respawns Actors "))
  (for _array_element (`self.RespawnQueue`)
    (set `local.DebugString` (`KismetStringLibrary.Concat_StrStr` (`local.DebugString`) (`KismetSystemLibrary.GetDisplayName` _array_element) " "))
    (bind _takenspawn (`self.SpawnActorFromPool` (struct) _array_element))
    (set `PlayerStart.PlayerStartTag` "None" _takenspawn))
  (`KismetArrayLibrary.Array_Clear` (`self.RespawnQueue`)))

(fn `HandleStartMatch`
  (if (`self.WereActorPoolsFilled`)
    (`self.SpawnActorsFromPool` (`self.ActorsPerTeam`) :!label _label)
    (else
      (bind _wassuccessful (`self.FillActorPools`))
      (bind _output_get (set `self.WereActorPoolsFilled` _wassuccessful))
      (if _output_get
        (goto _label)
        (else
          (`KismetSystemLibrary.PrintString` "*** Filling Actor Pool failed, no spawning possible ***"))))))

(fn `HandleUnitSpawned`
  (params (Actor :type "Actor Object Reference (by ref)"))
  (`KismetArrayLibrary.Array_AddUnique` (`self.ActorPoolBlue`) Actor)
  (bind _tagcontainer (message `GameplayTagAssetInterface.GetOwnedGameplayTags` Actor))
  (`|SwitchGameplayTagContainer` _tagcontainer
    (:`(GameplayTags=((TagName="Team.Blue")))`
      (`KismetArrayLibrary.Array_AddUnique` (`self.ActiveNormalActors`) (`local.Actor`)))
    (:`(GameplayTags=((TagName="Team.Red")))`
      (`KismetArrayLibrary.Array_AddUnique` (`self.ActiveExtendedActors`) (`local.Actor`)))))

(fn `PoolActor`
  (params (ActorToPool :type "Actor Object Reference") (Team :type "GameplayTagContainer Structure"))
  (returns (PooledActor :type "Actor Object Reference"))
  (locals (Actor :type "Actor Object Reference") (TeamComponent :type "/Game/00_Base/Systems/Components/WM_TeamComponent Object Reference") (LocalTeam :type "GameplayTagContainer Structure"))
  (bind (_returnvalue_location _returnvalue_rotation) (`KismetMathLibrary.BreakTransform` (`Actor.GetTransform` (`self.PoolSpawnBlue`))))
  (bind (_returnvalue_location_2 _returnvalue_rotation_2) (`KismetMathLibrary.BreakTransform` (`Actor.GetTransform` (`self.PoolSpawnRed`))))
  (set `local.LocalTeam` Team)
  (bind _output_get (set `local.Actor` ActorToPool))
  (`/Engine/EditorBlueprintResources/StandardMacros.IsValid` _output_get
    (:`Is Valid`
      (bind _output_get_2 (set `local.TeamComponent` (`Actor.GetComponentByClass` (`local.Actor`) "/Game/00_Base/Systems/Components/WM_TeamComponent.WM_TeamComponent_C")))
      (`/Engine/EditorBlueprintResources/StandardMacros.IsValid` _output_get_2
        (:`Is Valid`
          (set `local.LocalTeam` (`/Game/00_Base/Systems/Components/WM_TeamComponent.TeamTag` (`local.TeamComponent`))))
        (:`Is Not Valid`
          (`KismetSystemLibrary.PrintString` "*** Trying to Pool Actor without TeamComponent ***")
          (return null))))
    (:`Is Not Valid`
      (bind _spawnedactor (`self.SpawnNewActor` (`local.LocalTeam`)))
      (bind _output_get_3 (set `local.Actor` _spawnedactor))
      (`/Engine/EditorBlueprintResources/StandardMacros.IsValid` _output_get_3
        (:`Is Valid`
          _)
        (:`Is Not Valid`
          (`KismetSystemLibrary.PrintString` "*** Actor invalid and no new actor could be spawned, returning null ***")
          (return null)))))
  (`|SwitchGameplayTagContainer` (`local.LocalTeam`)
    (:`(GameplayTags=((TagName="Team.Blue")))`
      (`Actor.K2_SetActorTransform` (`local.Actor`) (`KismetMathLibrary.MakeTransform` _returnvalue_location _returnvalue_rotation) false true)
      (`KismetArrayLibrary.Array_AddUnique` (`self.ActorPoolBlue`) (`local.Actor`))
      (`KismetArrayLibrary.Array_RemoveItem` (`self.ActiveNormalActors`) (`local.Actor`)))
    (:`(GameplayTags=((TagName="Team.Red")))`
      (`Actor.K2_SetActorTransform` (`local.Actor`) (`KismetMathLibrary.MakeTransform` _returnvalue_location_2 _returnvalue_rotation_2) false true)
      (`KismetArrayLibrary.Array_AddUnique` (`self.ActorPoolRed`) (`local.Actor`))
      (`KismetArrayLibrary.Array_RemoveItem` (`self.ActiveExtendedActors`) (`local.Actor`))))
  (return (`local.Actor`)))

(fn `SetupNewTest`
  (params (NewBlueBT :type "BehaviorTree Object Reference") (NewRedBT :type "BehaviorTree Object Reference"))
  (set `self.TeamBlueBT` NewBlueBT)
  (set `self.TeamRedBT` NewRedBT)
  (`|ExecutionSequence`
    (:`then_0`
      (`|ExecutionSequence`
        (:`then_0`
          (for _array_element (`self.ActiveNormalActors`)
            (`Actor.K2_DestroyActor` _array_element))
          (`KismetArrayLibrary.Array_Clear` (`self.ActiveNormalActors`)))
        (:`then_1`
          (for _array_element_2 (`self.ActiveExtendedActors`)
            (`Actor.K2_DestroyActor` _array_element_2))
          (`KismetArrayLibrary.Array_Clear` (`self.ActiveExtendedActors`)))
        (:`then_2`
          (for _array_element_3 (`self.ActorPoolBlue`)
            (`Actor.K2_DestroyActor` _array_element_3))
          (`KismetArrayLibrary.Array_Clear` (`self.ActorPoolBlue`)))
        (:`then_3`
          (for _array_element_4 (`self.ActorPoolRed`)
            (`Actor.K2_DestroyActor` _array_element_4))
          (`KismetArrayLibrary.Array_Clear` (`self.ActorPoolRed`)))))
    (:`then_1`
      (set `self.WereActorPoolsFilled` false))
    (:`then_2`
      (`/Game/00_Base/WM_GameplayStatics.LogLine` (`KismetStringLibrary.Concat_StrStr` "========== " (`KismetSystemLibrary.GetDisplayName` (`self.TeamBlueBT`)) " vs. " (`KismetSystemLibrary.GetDisplayName` (`self.TeamRedBT`)) " ==========")))))

(fn `SpawnActorFromPool`
  (params (Team :type "GameplayTagContainer Structure") (ActorToRespawn :type "Actor Object Reference"))
  (returns (TakenSpawn :type "PlayerStart Object Reference"))
  (locals (Spawn :type "/Game/00_Base/WM_PlayerStart Object Reference") (Actor :type "Actor Object Reference") (TeamComponent :type "/Game/00_Base/Systems/Components/WM_TeamComponent Object Reference") (LocalTeam :type "GameplayTagContainer Structure"))
  (bind _returnvalue_location (`KismetMathLibrary.BreakTransform` (`Actor.GetTransform` (`local.Spawn`))))
  (set `local.LocalTeam` Team)
  (bind _output_get (set `local.Actor` ActorToRespawn))
  (`/Engine/EditorBlueprintResources/StandardMacros.IsValid` _output_get ; when valid, respawn specific actor, otherwise get actor from pool
    (:`Is Valid`
      (bind _output_get_2 (set `local.TeamComponent` (`Actor.GetComponentByClass` (`local.Actor`) "/Game/00_Base/Systems/Components/WM_TeamComponent.WM_TeamComponent_C")))
      (`/Engine/EditorBlueprintResources/StandardMacros.IsValid` _output_get_2
        (:`Is Valid`
          (set `local.LocalTeam` (`/Game/00_Base/Systems/Components/WM_TeamComponent.TeamTag` (`local.TeamComponent`)))
          (bind _output_get_3 (set `local.Spawn` (`self.FindSpawn` (`local.LocalTeam`)) :!label _label))
          (`/Engine/EditorBlueprintResources/StandardMacros.IsValid` _output_get_3
            (:`Is Valid`
              (set `PlayerStart.PlayerStartTag` "Taken" (`local.Spawn`))
              (`Actor.K2_SetActorTransform` (`local.Actor`) (`KismetMathLibrary.MakeTransform` _returnvalue_location) false true)
              (`|SwitchGameplayTagContainer` (`local.LocalTeam`)
                (:`(GameplayTags=((TagName="Team.Blue")))`
                  (`KismetArrayLibrary.Array_AddUnique` (`self.ActiveNormalActors`) (`local.Actor`))
                  (`KismetArrayLibrary.Array_RemoveItem` (`self.ActorPoolBlue`) (`local.Actor`)))
                (:`(GameplayTags=((TagName="Team.Red")))`
                  (`KismetArrayLibrary.Array_AddUnique` (`self.ActiveExtendedActors`) (`local.Actor`))
                  (`KismetArrayLibrary.Array_RemoveItem` (`self.ActorPoolRed`) (`local.Actor`))))
              (`self.ActorSpawned` (`local.Actor`))
              (return (`local.Spawn`)))
            (:`Is Not Valid`
              (`KismetSystemLibrary.PrintString` "*** No valid spawn found, not spawning and returning null ***"))))
        (:`Is Not Valid`
          (`KismetSystemLibrary.PrintString` "*** No TeamComponent found ***"))))
    (:`Is Not Valid`
      (`|SwitchGameplayTagContainer` (`local.LocalTeam`)
        (:`(GameplayTags=((TagName="Team.Blue")))`
          (if (> (`KismetArrayLibrary.Array_Length` (`self.ActorPoolBlue`)) 0)
            (set `local.Actor` (`|GetArrayItem` (`self.ActorPoolBlue`)))
            (`/Engine/EditorBlueprintResources/StandardMacros.IsValid` (`local.Actor`) :!label _label_2
              (:`Is Valid`
                (goto _label))
              (:`Is Not Valid`
                (`KismetSystemLibrary.PrintString` "*** Got invalid Actor from Actor Pool ***")))
            (else
              (`KismetSystemLibrary.PrintString` "*** Actor Pool empty, can't spawn Actor from pool ***" :!label _label_3))))
        (:`(GameplayTags=((TagName="Team.Red")))`
          (if (> (`KismetArrayLibrary.Array_Length` (`self.ActorPoolRed`)) 0)
            (set `local.Actor` (`|GetArrayItem` (`self.ActorPoolRed`)))
            (goto _label_2)
            (else
              (goto _label_3))))))))

(fn `SpawnActorsFromPool`
  (params (ActorsPerTeam :type Integer))
  (locals (TakenSpawns :type "Array of PlayerStart Object Reference"))
  (for _ (range 1 (+ ActorsPerTeam 1))
    (`|ExecutionSequence`
      (:`then_0`
        (bind _takenspawn (`self.SpawnActorFromPool` (struct :`GameplayTags` (struct :`(TagName` "Team.Blue")))))
        (`KismetArrayLibrary.Array_Add` (`local.TakenSpawns`) _takenspawn))
      (:`then_1`
        (bind _takenspawn_2 (`self.SpawnActorFromPool` (struct :`GameplayTags` (struct :`(TagName` "Team.Red")))))
        (`KismetArrayLibrary.Array_Add` (`local.TakenSpawns`) _takenspawn_2))))
  (for _array_element (`local.TakenSpawns`)
    (`/Engine/EditorBlueprintResources/StandardMacros.IsValid` _array_element
      (:`Is Valid`
        (set `PlayerStart.PlayerStartTag` "None" _array_element))))
  (`KismetArrayLibrary.Array_Clear` (`local.TakenSpawns`)))

(fn `SpawnNewActor`
  (params (Team :type "GameplayTagContainer Structure"))
  (returns (SpawnedActor :type "Actor Object Reference"))
  (locals (Actor :type "Actor Object Reference") (NameComponent :type "/Game/00_Base/Systems/Components/WM_NameComponent Object Reference") (TeamComponent :type "/Game/00_Base/Systems/Components/WM_TeamComponent Object Reference"))
  (bind _returnvalue_location (`KismetMathLibrary.BreakTransform` (`Actor.GetTransform` (`self.PoolSpawnBlue`))))
  (bind _returnvalue_location_2 (`KismetMathLibrary.BreakTransform` (`Actor.GetTransform` (`self.PoolSpawnRed`))))
  (`|SwitchGameplayTagContainer` Team
    (:`(GameplayTags=((TagName="Team.Blue")))`
      (bind _returnvalue (`AIBlueprintHelperLibrary.SpawnAIFromClass` "/Game/03_Units/WM_Actor.WM_Actor_C" (`self.TeamBlueBT`) _returnvalue_location (struct) true))
      (set `local.Actor` _returnvalue))
    (:`(GameplayTags=((TagName="Team.Red")))`
      (bind _returnvalue_2 (`AIBlueprintHelperLibrary.SpawnAIFromClass` "/Game/03_Units/WM_Actor.WM_Actor_C" (`self.TeamRedBT`) _returnvalue_location_2 (struct) true))
      (set `local.Actor` _returnvalue_2)))
  (bind _output_get (set `local.NameComponent` (`Actor.GetComponentByClass` (`local.Actor`) "/Game/00_Base/Systems/Components/WM_NameComponent.WM_NameComponent_C")))
  (`/Engine/EditorBlueprintResources/StandardMacros.IsValid` _output_get
    (:`Is Valid`
      _)
    (:`Is Not Valid`
      (`KismetSystemLibrary.PrintString` "*** Actor has no NameComponent ***")))
  (bind _output_get_2 (set `local.TeamComponent` (`Actor.GetComponentByClass` (`local.Actor`) "/Game/00_Base/Systems/Components/WM_TeamComponent.WM_TeamComponent_C")))
  (`/Engine/EditorBlueprintResources/StandardMacros.IsValid` _output_get_2
    (:`Is Valid`
      (`/Game/00_Base/Systems/Components/WM_TeamComponent.SetTeam` (`local.TeamComponent`) (`local.Team`)))
    (:`Is Not Valid`
      (`KismetSystemLibrary.PrintString` "*** Actor has no TeamComponent ***")))
  (return (`local.Actor`)))