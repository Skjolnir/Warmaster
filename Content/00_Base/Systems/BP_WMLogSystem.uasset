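; BP_WMLogSystem is a logging Blueprint that records a play session and saves it as a Warmaster log text file.
; BeginPlay passes a date and time stamped start line to LogLine.
; EndPlay logs a matching end line, then writes the LinesToLog array to a .txt file named with the current date and time.
; The file is written only at EndPlay.
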(event `self.ReceiveBeginPlay`
  (bind (_returnvalue_year _returnvalue_month _returnvalue_day _returnvalue_hour _returnvalue_minute _returnvalue_second) (`KismetMathLibrary.BreakDateTime` (`KismetMathLibrary.Now`)))
  (`/Game/00_Base/WM_GameplayStatics.LogLine` (`KismetStringLibrary.Concat_StrStr` "Start Date: " (`KismetStringLibrary.Conv_IntToString` _returnvalue_year) "-" (`KismetStringLibrary.Conv_IntToString` _returnvalue_month) "-" (`KismetStringLibrary.Conv_IntToString` _returnvalue_day) " Time: " (`KismetStringLibrary.Conv_IntToString` _returnvalue_hour) "-" (`KismetStringLibrary.Conv_IntToString` _returnvalue_minute) "-" (`KismetStringLibrary.Conv_IntToString` _returnvalue_second))))

(event `self.ReceiveEndPlay`
  (params (EndPlayReason :type "EEndPlayReason Enum" :default "Destroyed"))
  (bind (_returnvalue_year _returnvalue_month _returnvalue_day _returnvalue_hour _returnvalue_minute _returnvalue_second) (`KismetMathLibrary.BreakDateTime` (`KismetMathLibrary.Now`)))
  (bind (_returnvalue_year_2 _returnvalue_month_2 _returnvalue_day_2 _returnvalue_hour_2 _returnvalue_minute_2 _returnvalue_second_2) (`KismetMathLibrary.BreakDateTime` (`KismetMathLibrary.Now`)))
  (`/Game/00_Base/WM_GameplayStatics.LogLine` (`KismetStringLibrary.Concat_StrStr` "End Date: " (`KismetStringLibrary.Conv_IntToString` _returnvalue_year) "-" (`KismetStringLibrary.Conv_IntToString` _returnvalue_month) "-" (`KismetStringLibrary.Conv_IntToString` _returnvalue_day) " Time: " (`KismetStringLibrary.Conv_IntToString` _returnvalue_hour) "-" (`KismetStringLibrary.Conv_IntToString` _returnvalue_minute) "-" (`KismetStringLibrary.Conv_IntToString` _returnvalue_second)))
  (`WMUtilities.FileSaveStringArray` (`self.LinesToLog`) (`KismetStringLibrary.Concat_StrStr` "Warmaster Log " (`KismetStringLibrary.Concat_StrStr` (`KismetStringLibrary.Conv_IntToString` _returnvalue_year_2) "-" (`KismetStringLibrary.Conv_IntToString` _returnvalue_month_2) "-" (`KismetStringLibrary.Conv_IntToString` _returnvalue_day_2) " - " (`KismetStringLibrary.Conv_IntToString` _returnvalue_hour_2) "-" (`KismetStringLibrary.Conv_IntToString` _returnvalue_minute_2) "-" (`KismetStringLibrary.Conv_IntToString` _returnvalue_second_2)) ".txt")))