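; BP_WMDamageSystem resolves attacks between units and initializes the health and armor of spawned actors.
; It binds its attack event and the spawn event of the GameMode's BP_WMUnitSystem.
; Viable attacks draw a team-colored debug line and apply the attacker's damage to armor first, passing overkill to health and reporting kills to the unit system.
; Spawning restores full health and zeroes armor; HandleActorDied is an empty stub.
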(event `self.ReceiveBeginPlay`
  (set `self.UnitSystem` (`Actor.GetComponentByClass` (`GameplayStatics.GetGameMode`) "/Game/00_Base/Systems/BP_WMUnitSystem.BP_WMUnitSystem_C"))
  (add `self.AttackTarget` (delegate `Event Attack Target`))
  (add `WMUnitSystem.ActorSpawned` (`self.UnitSystem`) (delegate `Event Actor Spawned`)))

(event `Event Attack Target` :!signature `self.AttackTarget`
  (params (Actor :type "Actor Object Reference") (Target :type "Actor Object Reference"))
  (`self.HandleAttack` Actor Target))

(event `Event Actor Spawned`
  (params (Actor :type "Actor Object Reference"))
  (`self.HandleActorSpawned` Actor))

(fn `HandleActorDied`
  (params (Actor :type "Actor Object Reference")))

(fn `HandleActorSpawned`
  (params (Actor :type "Actor Object Reference"))
  (locals (HealthComponent :type "/Game/00_Base/Systems/Components/WM_HealthComponent Object Reference") (ArmorComponent :type "/Game/00_Base/Systems/Components/WM_ArmorComponent Object Reference"))
  (bind _output_get (set `local.HealthComponent` (`Actor.GetComponentByClass` Actor "/Game/00_Base/Systems/Components/WM_HealthComponent.WM_HealthComponent_C")))
  (`/Engine/EditorBlueprintResources/StandardMacros.IsValid` _output_get
    (:`Is Valid`
      (bind _output_get_2 (set `local.ArmorComponent` (`Actor.GetComponentByClass` (`local.Actor`) "/Game/00_Base/Systems/Components/WM_ArmorComponent.WM_ArmorComponent_C")))
      (`/Engine/EditorBlueprintResources/StandardMacros.IsValid` _output_get_2
        (:`Is Valid`
          (set `/Game/00_Base/Systems/Components/WM_HealthComponent.CurrentHealth` (`/Game/00_Base/Systems/Components/WM_HealthComponent.MaxHealth` (`local.HealthComponent`)) (`local.HealthComponent`))
          (set `/Game/00_Base/Systems/Components/WM_HealthComponent.IsAlive` true (`local.HealthComponent`))
          (set `/Game/00_Base/Systems/Components/WM_ArmorComponent.CurrentArmor` 0.0 (`local.ArmorComponent`)))
        (:`Is Not Valid`
          (`KismetSystemLibrary.PrintString` "*** Spawned Actor has no Armor Component ***"))))
    (:`Is Not Valid`
      (`KismetSystemLibrary.PrintString` "*** Spawned Actor has no Health Component ***"))))

(fn `HandleAttack`
  (params (Actor :type "Actor Object Reference") (Target :type "Actor Object Reference"))
  (locals (RealDamage :type "Float (double-precision)") (DebugString :type String) (DamageComponent :type "/Game/00_Base/Systems/Components/WM_DamageComponent Object Reference") (ArmorComponent :type "/Game/00_Base/Systems/Components/WM_ArmorComponent Object Reference") (HealthComponent :type "/Game/00_Base/Systems/Components/WM_HealthComponent Object Reference") (TeamComponent :type "/Game/00_Base/Systems/Components/WM_TeamComponent Object Reference"))
  (if (`/Game/00_Base/WM_GameplayStatics.IsTargetActorViable` Actor Target)
    (bind _output_get (set `local.TeamComponent` (`Actor.GetComponentByClass` (`local.Actor`) "/Game/00_Base/Systems/Components/WM_TeamComponent.WM_TeamComponent_C")))
    (`/Engine/EditorBlueprintResources/StandardMacros.IsValid` _output_get
      (:`Is Valid`
        (`KismetSystemLibrary.DrawDebugLine` (`Actor.K2_GetActorLocation` (`local.Actor`)) (`Actor.K2_GetActorLocation` (`local.Target`)) (`/Game/00_Base/Systems/Components/WM_TeamComponent.TeamColor` (`local.TeamComponent`)) 0.25 10.0))
      (:`Is Not Valid`
        (`KismetSystemLibrary.PrintString` "*** No TeamComponent found ***")))
    (bind _output_get_2 (set `local.DamageComponent` (`Actor.GetComponentByClass` (`local.Actor`) "/Game/00_Base/Systems/Components/WM_DamageComponent.WM_DamageComponent_C")))
    (`/Engine/EditorBlueprintResources/StandardMacros.IsValid` _output_get_2
      (:`Is Valid`
        (set `local.RealDamage` (* (`/Game/00_Base/Systems/Components/WM_DamageComponent.Damage` (`local.DamageComponent`)) -1.0)) ; Damage comes in positive, health and armor components work with damage = negative change
        (bind _output_get_3 (set `local.HealthComponent` (`Actor.GetComponentByClass` (`local.Target`) "/Game/00_Base/Systems/Components/WM_HealthComponent.WM_HealthComponent_C")))
        (`/Engine/EditorBlueprintResources/StandardMacros.IsValid` _output_get_3
          (:`Is Valid`
            (bind _output_get_4 (set `local.ArmorComponent` (`Actor.GetComponentByClass` (`local.Target`) "/Game/00_Base/Systems/Components/WM_ArmorComponent.WM_ArmorComponent_C")))
            (`/Engine/EditorBlueprintResources/StandardMacros.IsValid` _output_get_4
              (:`Is Valid`
                (if (`/Game/00_Base/Systems/Components/WM_ArmorComponent.HasArmor` (`local.ArmorComponent`))
                  ;[1 1 1] Armor Handling
                  (bind (_hasarmor _overkill) (`/Game/00_Base/Systems/Components/WM_ArmorComponent.ChangeArmorBy` (`local.ArmorComponent`) (`local.RealDamage`)))
                  (if (not _hasarmor)
                    (set `local.RealDamage` _overkill) ; overkill becomes damage to health component
                    (bind _alive (`/Game/00_Base/Systems/Components/WM_HealthComponent.ChangeHealthBy` (`local.HealthComponent`) (`local.RealDamage`) :!label _label))
                    (if (not _alive)
                      (`WMUnitSystem.ActorKilled` (`self.UnitSystem`) (`local.Target`) (`local.Actor`))))
                  (else
                    (goto _label))))
              (:`Is Not Valid`
                (set `local.DebugString` "*** Target has no \"WM_ArmorComponent\" ***")
                (goto _label))))
          (:`Is Not Valid`
            (set `local.DebugString` "*** Target has no \"WM_HealthComponent\" ***"))))
      (:`Is Not Valid`
        (set `local.DebugString` "*** Attacker has no \"WM_DamageComponent\" ***")))
    (else
      (set `local.DebugString` "*** Attack failed due to \"IsViableTarget\" result ***"))))