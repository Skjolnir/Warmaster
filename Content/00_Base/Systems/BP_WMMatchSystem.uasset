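; Match system that automates repeated AI-versus-AI team matches to compare two behavior trees.
; It listens for team wins from BP_WMScoreSystem on the game mode, restarting matches after short delays until MaxMatches is reached, then logging each team's wins and kills.
; Each next test resets stats and has BP_WMUnitSystem assign trees from a fixed schedule of repeated pairings, swapped sides and mirror matchups, quitting once it runs out.
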(event `self.ReceiveBeginPlay`
  (`|ExecutionSequence`
    (:`then_0`
      (bind _output_get (set `self.ScoreSystem` (`Actor.GetComponentByClass` (`GameplayStatics.GetGameMode`) "/Game/00_Base/Systems/BP_WMScoreSystem.BP_WMScoreSystem_C")))
      (`/Engine/EditorBlueprintResources/StandardMacros.IsValid` _output_get
        (:`Is Valid`
          (add `WMScoreSystem.TeamWins` (`self.ScoreSystem`) (delegate `Event Team Wins`)))
        (:`Is Not Valid`
          (`KismetSystemLibrary.PrintString` "*** Game Mode has no \"WMScoreSystem\" component ***"))))
    (:`then_1`
      (bind _output_get_2 (set `self.UnitSystem` (`Actor.GetComponentByClass` (`GameplayStatics.GetGameMode`) "/Game/00_Base/Systems/BP_WMUnitSystem.BP_WMUnitSystem_C")))
      (`/Engine/EditorBlueprintResources/StandardMacros.IsValid` _output_get_2
        (:`Is Not Valid`
          (`KismetSystemLibrary.PrintString` "*** Game Mode has no \"WMUnitSystem\" component ***"))))
    (:`then_2`
      (add `self.SetupNextTest` (delegate `Setup Next Test Event`)))))

(event `Event Team Wins`
  (params (Team :type "ETeam Enum" :default "T_NormalBlue"))
  (`/Engine/EditorBlueprintResources/StandardMacros.IncrementInt` (`self.MatchCount`)
    (:`  `
      (`KismetSystemLibrary.Delay` 2.0)
      (`self.EndMatch`)
      (`KismetSystemLibrary.PrintString` (`KismetStringLibrary.Concat_StrStr` (`KismetStringLibrary.Conv_IntToString` (`self.MatchCount`)) " matches done."))
      (if (< (`self.MatchCount`) (`self.MaxMatches`))
        (`KismetSystemLibrary.Delay` 5.0)
        (`self.StartMatch`)
        (else
          (`/Game/00_Base/WM_GameplayStatics.LogLine` (`KismetStringLibrary.Concat_StrStr` "Test Complete - Blue: " (`KismetStringLibrary.Conv_IntToString` (`/Game/00_Base/Systems/BP_WMScoreSystem.ScoreBlue` (`self.ScoreSystem`))) " wins, " (`KismetStringLibrary.Conv_IntToString` (`/Game/00_Base/Systems/BP_WMScoreSystem.TotalKillsBlue` (`self.ScoreSystem`))) " kills - Red: " (`KismetStringLibrary.Conv_IntToString` (`/Game/00_Base/Systems/BP_WMScoreSystem.ScoreRed` (`self.ScoreSystem`))) " wins, " (`KismetStringLibrary.Conv_IntToString` (`/Game/00_Base/Systems/BP_WMScoreSystem.TotalKillsRed` (`self.ScoreSystem`))) " kills"))
          (`self.SetupNextTest`))))))

(event `Setup Next Test Event`
  (bind _testaione (`self.TestAIOne`))
  (bind _testaitwo (`self.TestAITwo`))
  (`|ExecutionSequence`
    (:`then_0`
      (`/Game/00_Base/Systems/BP_WMScoreSystem.Reset Stats` (`self.ScoreSystem`)))
    (:`then_1`
      (set `self.MatchCount` 0))
    (:`then_2`
      (switch `int` (`self.TestCount`)
        (:`Default`
          (`KismetSystemLibrary.QuitGame` null "Quit"))
        (:`0`
          (`/Game/00_Base/Systems/BP_WMUnitSystem.SetupNewTest` (`self.UnitSystem`) (`self.TestAIOne`) (`self.TestAITwo`) :!label _label))
        (:`1`
          (goto _label))
        (:`2`
          (goto _label))
        (:`3`
          (`/Game/00_Base/Systems/BP_WMUnitSystem.SetupNewTest` (`self.UnitSystem`) (`self.TestAITwo`) (`self.TestAIOne`) :!label _label_2))
        (:`4`
          (goto _label_2))
        (:`5`
          (goto _label_2))
        (:`6`
          (`/Game/00_Base/Systems/BP_WMUnitSystem.SetupNewTest` (`self.UnitSystem`) _testaione _testaione))
        (:`7`
          (`/Game/00_Base/Systems/BP_WMUnitSystem.SetupNewTest` (`self.UnitSystem`) _testaitwo _testaitwo))))
    (:`then_3`
      (`/Engine/EditorBlueprintResources/StandardMacros.IncrementInt` (`self.TestCount`)))
    (:`then_4`
      (`KismetSystemLibrary.Delay` 5.0)
      (`self.StartMatch`))))