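; Score system that tracks kills and round wins for the Blue and Red teams.
; On BeginPlay it binds to the ActorKilled dispatcher of the game mode's BP_WMUnitSystem component and credits each kill via the killer's WM_TeamComponent tag.
; Reaching KillsForWin fires its TeamWins dispatcher, whose own handler clears round kills and increments that team's score.
; Total kills persist across rounds until ResetStats zeroes all counters.
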(event `self.ReceiveBeginPlay`
  (bind _output_get (set `self.UnitSystem` (`Actor.GetComponentByClass` (`GameplayStatics.GetGameMode`) "/Game/00_Base/Systems/BP_WMUnitSystem.BP_WMUnitSystem_C")))
  (`/Engine/EditorBlueprintResources/StandardMacros.IsValid` _output_get
    (:`Is Valid`
      (add `WMUnitSystem.ActorKilled` (`self.UnitSystem`) (delegate `Event Actor Killed`))
      (add `self.TeamWins` (delegate `Event Team Wins`)))
    (:`Is Not Valid`
      (`KismetSystemLibrary.PrintString` "*** Gamemode has no \"WM_UnitSystem\" component ***"))))

(event `Event Actor Killed`
  (params (Actor :type "Actor Object Reference") (Killer :type "Actor Object Reference"))
  (`|SwitchGameplayTagContainer` (`/Game/00_Base/Systems/Components/WM_TeamComponent.TeamTag` (`Actor.GetComponentByClass` Killer "/Game/00_Base/Systems/Components/WM_TeamComponent.WM_TeamComponent_C"))
    (:`(GameplayTags=((TagName="Team.Blue")))`
      (`/Engine/EditorBlueprintResources/StandardMacros.IncrementInt` (`self.KillsBlue`)
        (:`  `
          (`/Engine/EditorBlueprintResources/StandardMacros.IncrementInt` (`self.TotalKillsBlue`)
            (:`  `
              (if (>= (`self.KillsBlue`) (`self.KillsForWin`))
                ;[0 0.35 1] Blue Wins
                (`self.TeamWins` "T_NormalBlue")))))))
    (:`(GameplayTags=((TagName="Team.Red")))`
      (`/Engine/EditorBlueprintResources/StandardMacros.IncrementInt` (`self.KillsRed`)
        (:`  `
          (`/Engine/EditorBlueprintResources/StandardMacros.IncrementInt` (`self.TotalKillsRed`)
            (:`  `
              (if (>= (`self.KillsRed`) (`self.KillsForWin`))
                ;[1 0.073 0] Red Wins
                (`self.TeamWins` "T_ExtendedRed")))))))))

(event `Event Team Wins` :!signature `self.TeamWins`
  (params (Team :type "ETeam Enum" :default "T_NormalBlue"))
  (set `self.KillsRed` 0)
  (set `self.KillsBlue` 0)
  (switch `ETeam` Team
    (:`T_NormalBlue`
      (`/Engine/EditorBlueprintResources/StandardMacros.IncrementInt` (`self.ScoreBlue`)))
    (:`T_ExtendedRed`
      (`/Engine/EditorBlueprintResources/StandardMacros.IncrementInt` (`self.ScoreRed`)))))

(event `Reset Stats`
  (set `self.KillsBlue` 0)
  (set `self.KillsRed` 0)
  (set `self.ScoreBlue` 0)
  (set `self.ScoreRed` 0)
  (set `self.TotalKillsBlue` 0)
  (set `self.TotalKillsRed` 0))